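; Pressure-button actor, apparently the third of a set, that reports to the player's KnightBP whether its trigger Box is overlapped.
; BeginPlay caches the player pawn as KnightBP; overlap begin and end set and clear its ButtonThree flag, without filtering the overlapping actor.
; Each event also finds the first Text actor and shifts its Text component along relative X, out on begin and back to zero on end.
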(event `self.ReceiveBeginPlay`
  (bind _asknight_bp (cast `/Game/Blueprints/KnightBP` (`GameplayStatics.GetPlayerPawn` 0)))
  (set `self.As Knight BP` _asknight_bp))

(event `self.Box.OnComponentBeginOverlap`
  (params (OverlappedComponent :type "PrimitiveComponent Object Reference") (OtherActor :type "Actor Object Reference") (OtherComp :type "PrimitiveComponent Object Reference") (OtherBodyIndex :type Integer) (bFromSweep :type Boolean) (SweepResult :type "HitResult Structure (by ref)"))
  (set `/Game/Blueprints/KnightBP.ButtonThree` true (`self.As Knight BP`))
  (bind _outactors (`GameplayStatics.GetAllActorsOfClass` "/Game/Blueprints/Text.Text_C"))
  (bind _text (`/Game/Blueprints/Text.Text` (`|GetArrayItem` _outactors)))
  (bind _returnvalue (`SceneComponent.GetRelativeTransform` _text))
  (`SceneComponent.K2_SetRelativeTransform` _text (`KismetMathLibrary.MakeTransform` (`KismetMathLibrary.MakeVector` 5.0 (.y (.location _returnvalue)) (.z (.location _returnvalue))) (.rotation _returnvalue) (.scale _returnvalue)) false false))

(event `self.Box.OnComponentEndOverlap`
  (params (OverlappedComponent :type "PrimitiveComponent Object Reference") (OtherActor :type "Actor Object Reference") (OtherComp :type "PrimitiveComponent Object Reference") (OtherBodyIndex :type Integer))
  (set `/Game/Blueprints/KnightBP.ButtonThree` false (`self.As Knight BP`))
  (bind _outactors (`GameplayStatics.GetAllActorsOfClass` "/Game/Blueprints/Text.Text_C"))
  (bind _text (`/Game/Blueprints/Text.Text` (`|GetArrayItem` _outactors)))
  (bind _returnvalue (`SceneComponent.GetRelativeTransform` _text))
  (`SceneComponent.K2_SetRelativeTransform` _text (`KismetMathLibrary.MakeTransform` (`KismetMathLibrary.MakeVector` 0.0 (.y (.location _returnvalue)) (.z (.location _returnvalue))) (.rotation _returnvalue) (.scale _returnvalue)) false false))

(fn `UserConstructionScript`)