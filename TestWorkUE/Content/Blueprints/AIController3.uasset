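; AI controller that shuttles its pawn back and forth between two level TargetPoints.
; Each Tick fetches all TargetPoints and picks the third or fourth by array index, based on a Forward flag.
; It issues a MoveToLocation, waits on a short Delay, then stops movement and flips the flag, so legs are timed rather than driven by arrival.
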(event `self.ReceiveTick`
  (params (DeltaSeconds :type "Float (single-precision)"))
  ;[1 1 1] ИИ Движение вперёд и назад
  (bind _outactors (`GameplayStatics.GetAllActorsOfClass` "/Script/Engine.TargetPoint"))
  (if (`self.Forward`)
    (`self.MoveToLocation` (`self.K2_GetActorLocation` (`|GetArrayItem` _outactors 2)) 30.0 true true false true null)
    (`KismetSystemLibrary.Delay` 1.0)
    (`self.StopMovement`)
    (set `self.Forward` false)
    (if true
      _)
    (else
      (`self.MoveToLocation` (`self.K2_GetActorLocation` (`|GetArrayItem` _outactors 3)) -1.0 false true false true null)
      (`KismetSystemLibrary.Delay` 0.5)
      (`self.StopMovement`)
      (set `self.Forward` true))))

(fn `UserConstructionScript`)