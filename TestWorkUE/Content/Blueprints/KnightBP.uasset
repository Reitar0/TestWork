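; Player knight character with axis-driven movement and camera look that can press three buttons to summon NPCs.
; BeginPlay caches the locations of the Cube1, Cube2 and Cube3 actors as spawn points.
; E checks each button flag, plays a push montage and sound, and shifts that button's cylinder.
; After a delay, it spawns the matching NPC and a Fire effect at its cube, resets the cylinder and plays a spell sound.
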(event `self.ReceiveBeginPlay`
  ;[1 1 1] Переменные
  (bind _outactors (`GameplayStatics.GetAllActorsOfClass` "/Game/Blueprints/Cube1.Cube1_C"))
  (set `self.BoxOne` (`self.K2_GetActorLocation` (`|GetArrayItem` _outactors)))
  (bind _outactors_2 (`GameplayStatics.GetAllActorsOfClass` "/Game/Blueprints/Cube2.Cube2_C"))
  (set `self.BoxTwo` (`self.K2_GetActorLocation` (`|GetArrayItem` _outactors_2)))
  (bind _outactors_3 (`GameplayStatics.GetAllActorsOfClass` "/Game/Blueprints/Cube3.Cube3_C"))
  (set `self.BowThree` (`self.K2_GetActorLocation` (`|GetArrayItem` _outactors_3))))

(event `InputAxis|MoveForward`
  (params (AxisValue :type "Float (single-precision)"))
  (bind (_returnvalue_roll _returnvalue_pitch _returnvalue_yaw) (`KismetMathLibrary.BreakRotator` (`self.GetControlRotation`)))
  ;[1 1 1] Идти вперёд
  (`self.AddMovementInput` (`KismetMathLibrary.GetForwardVector` (`KismetMathLibrary.MakeRotator` 0.0 0.0 _returnvalue_yaw)) AxisValue))

(event `InputAxis|MoveRight`
  (params (AxisValue :type "Float (single-precision)"))
  (bind (_returnvalue_roll _returnvalue_pitch _returnvalue_yaw) (`KismetMathLibrary.BreakRotator` (`self.GetControlRotation`)))
  ;[1 1 1] Идти в сторону
  (`self.AddMovementInput` (`KismetMathLibrary.GetRightVector` (`KismetMathLibrary.MakeRotator` _returnvalue_roll 0.0 _returnvalue_yaw)) AxisValue))

(event `InputAxis|Turn`
  (params (AxisValue :type "Float (single-precision)"))
  ;[1 1 1] Поворот камеры
  (`self.AddControllerYawInput` AxisValue))

(event `InputAxis|LookUp`
  (params (AxisValue :type "Float (single-precision)"))
  ;[1 1 1] Поворот камеры
  (`self.AddControllerPitchInput` AxisValue))

(event `self.ReceiveTick`
  (params (DeltaSeconds :type "Float (single-precision)")))

(event `Key|E`
  (params (Key :type "Key Structure"))
  (bind _boxone (`self.BoxOne`))
  (:`Pressed`
    (if (`self.ButtonOne`)
      (`|PlayMontage` (`self.Mesh`) "/Game/Character/Animations/Push.Push" 8.0
        (:`then`
          (`GameplayStatics.PlaySound2D` "/Game/Sound/Special_Attacks/cue/Special_Attack_02_Cue.Special_Attack_02_Cue" 1.0 1.0 0.0 null null)
          (bind _outactors (`GameplayStatics.GetAllActorsOfClass` "/Game/Blueprints/ButtonBP.ButtonBP_C"))
          (bind _cylinder (`/Game/Blueprints/ButtonBP.Cylinder` (`|GetArrayItem` _outactors)))
          (bind (_returnvalue_location _returnvalue_rotation _returnvalue_scale) (`KismetMathLibrary.BreakTransform` (`SceneComponent.GetRelativeTransform` _cylinder)))
          (`SceneComponent.K2_SetRelativeTransform` _cylinder (`KismetMathLibrary.MakeTransform` (-10.0 0.0 0.0) _returnvalue_rotation _returnvalue_scale) false false)
          (`KismetSystemLibrary.Delay` 1.5)
          (`/Engine/EditorBlueprintResources/StandardMacros.IsValid` "/Game/Blueprints/NPC1.NPC1"
            (:`Is Valid`
              (`|SpawnActorFromClass` "/Game/Blueprints/NPC1.NPC1_C" (`KismetMathLibrary.MakeTransform` _boxone (struct :`Yaw` 45.900002)) "AlwaysSpawn" "OverrideRootScale" null null)
              (`SceneComponent.K2_SetRelativeTransform` _cylinder (`KismetMathLibrary.MakeTransform` (0.0 0.0 0.0) _returnvalue_rotation _returnvalue_scale) false false)
              (`GameplayStatics.PlaySound2D` "/Game/Sound/Elements___School/Arcane/wav/Arcane_Spell_2.Arcane_Spell_2" 1.0 1.0 0.0 null null)
              (`|SpawnActorFromClass` "/Game/Blueprints/Fire.Fire_C" (`KismetMathLibrary.MakeTransform` _boxone) "Undefined" "OverrideRootScale" null null))))))))

(event `Key|E`
  (params (Key :type "Key Structure"))
  (bind _boxtwo (`self.BoxTwo`))
  (:`Pressed`
    (if (`self.ButtonTwo`)
      (`|PlayMontage` (`self.Mesh`) "/Game/Character/Animations/Push.Push" 8.0
        (:`then`
          (`GameplayStatics.PlaySound2D` "/Game/Sound/Special_Attacks/cue/Special_Attack_02_Cue.Special_Attack_02_Cue" 1.0 1.0 0.0 null null)
          (bind _outactors (`GameplayStatics.GetAllActorsOfClass` "/Game/Blueprints/ButtonBP_2.ButtonBP_2_C"))
          (bind _cylinder (`/Game/Blueprints/ButtonBP_2.Cylinder` (`|GetArrayItem` _outactors)))
          (bind (_returnvalue_location _returnvalue_rotation _returnvalue_scale) (`KismetMathLibrary.BreakTransform` (`SceneComponent.GetRelativeTransform` _cylinder)))
          (`SceneComponent.K2_SetRelativeTransform` _cylinder (`KismetMathLibrary.MakeTransform` (-10.0 0.0 0.0) _returnvalue_rotation _returnvalue_scale) false false)
          (`KismetSystemLibrary.Delay` 1.5)
          (`/Engine/EditorBlueprintResources/StandardMacros.IsValid` "/Game/Blueprints/NPC2.NPC2"
            (:`Is Valid`
              (`|SpawnActorFromClass` "/Game/Blueprints/NPC2.NPC2_C" (`KismetMathLibrary.MakeTransform` _boxtwo (struct :`Yaw` 45.900002)) "AlwaysSpawn" "OverrideRootScale" null null)
              (`SceneComponent.K2_SetRelativeTransform` _cylinder (`KismetMathLibrary.MakeTransform` (0.0 0.0 0.0) _returnvalue_rotation _returnvalue_scale) false false)
              (`GameplayStatics.PlaySound2D` "/Game/Sound/Elements___School/Arcane/cue/Arcane_Spell_10_2_Cue.Arcane_Spell_10_2_Cue" 1.0 1.0 0.0 null null)
              (`|SpawnActorFromClass` "/Game/Blueprints/Fire.Fire_C" (`KismetMathLibrary.MakeTransform` _boxtwo) "Undefined" "OverrideRootScale" null null))))))))

(event `Key|E`
  (params (Key :type "Key Structure"))
  (bind _bowthree (`self.BowThree`))
  (:`Pressed`
    (if (`self.ButtonThree`)
      (`|PlayMontage` (`self.Mesh`) "/Game/Character/Animations/Push.Push" 8.0
        (:`then`
          (`GameplayStatics.PlaySound2D` "/Game/Sound/Special_Attacks/cue/Special_Attack_02_Cue.Special_Attack_02_Cue" 1.0 1.0 0.0 null null)
          (bind _outactors (`GameplayStatics.GetAllActorsOfClass` "/Game/Blueprints/ButtonBP_3.ButtonBP_3_C"))
          (bind _cylinder (`/Game/Blueprints/ButtonBP_3.Cylinder` (`|GetArrayItem` _outactors)))
          (bind (_returnvalue_location _returnvalue_rotation _returnvalue_scale) (`KismetMathLibrary.BreakTransform` (`SceneComponent.GetRelativeTransform` _cylinder)))
          (`SceneComponent.K2_SetRelativeTransform` _cylinder (`KismetMathLibrary.MakeTransform` (-10.0 0.0 0.0) _returnvalue_rotation _returnvalue_scale) false false)
          (`KismetSystemLibrary.Delay` 1.5)
          (`/Engine/EditorBlueprintResources/StandardMacros.IsValid` "/Game/Blueprints/NPC3.NPC3"
            (:`Is Valid`
              (`|SpawnActorFromClass` "/Game/Blueprints/NPC3.NPC3_C" (`KismetMathLibrary.MakeTransform` _bowthree (struct :`Yaw` 45.900002)) "AlwaysSpawn" "OverrideRootScale" null null)
              (`SceneComponent.K2_SetRelativeTransform` _cylinder (`KismetMathLibrary.MakeTransform` (0.0 0.0 0.0) _returnvalue_rotation _returnvalue_scale) false false)
              (`GameplayStatics.PlaySound2D` "/Game/Sound/Elements___School/Arcane/cue/Arcane_Spell_7_2_Cue.Arcane_Spell_7_2_Cue" 1.0 1.0 0.0 null null)
              (`|SpawnActorFromClass` "/Game/Blueprints/Fire.Fire_C" (`KismetMathLibrary.MakeTransform` _bowthree) "Undefined" "OverrideRootScale" null null))))))))

(fn `UserConstructionScript`)