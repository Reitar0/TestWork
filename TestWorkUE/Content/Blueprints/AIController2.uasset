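; AI controller that moves its pawn toward a level TargetPoint in a stop-and-go pattern.
; Tick gathers all TargetPoint actors, and the Run flag selects between moving to the one at index 1 and pausing.
; Latent Delays time each phase before StopMovement or the flag flip, then wire back into the branch to repeat the cycle, alongside re-entry from every Tick.
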(event `self.ReceiveTick`
  (params (DeltaSeconds :type "Float (single-precision)"))
  ;[1 1 1] ИИ Движение с остановкой
  (bind _outactors (`GameplayStatics.GetAllActorsOfClass` "/Script/Engine.TargetPoint"))
  (if (`self.Run`) :!label _label
    (`AIBlueprintHelperLibrary.SimpleMoveToLocation` self (`self.K2_GetActorLocation` (`|GetArrayItem` _outactors 1)))
    (`KismetSystemLibrary.Delay` 1.0)
    (`self.StopMovement`)
    (set `self.Run` false)
    (goto _label)
    (else
      (`KismetSystemLibrary.Delay` 0.5)
      (set `self.Run` true)
      (goto _label))))

(fn `UserConstructionScript`)